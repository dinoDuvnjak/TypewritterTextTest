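; HUD Blueprint that starts a dialogue screen with typed-out text when play begins.
; On BeginPlay it blocking-loads a DialogueDataAsset and reads its DialogueSequence, printing an error if that is empty.
; Otherwise an init event creates WBP_PrimaryLayout, gives it UI-only input focus, and passes it the first sequence entry with a typing interval.
; An async load node is left unconnected.
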(event Custom|CE_OnInitDialogue
  (bind _returnvalue (Game|GetPlayerController 0))
  (bind _returnvalue_2 (UserInterface|CreateWidget "/Game/Widgets/WBP_PrimaryLayout.WBP_PrimaryLayout_C" _returnvalue))
  (UserInterface|Viewport|AddtoViewport _returnvalue_2 0)
  (Input|SetInputModeUIOnly _returnvalue _returnvalue_2 "DoNotLock" false)
  (Class|DialogueWidget|StartDialogue _returnvalue_2 (Utilities|Array|Get(acopy) (Variables|Default|GetDialogue%20Sequence)) 0.01))

(event EventBeginPlay
  (bind _returnvalue (Utilities|LoadAssetBlocking (Variables|Default|GetDialogueSequenceDataAsset)))
  (bind _asdialogue_data_asset (Utilities|Casting|CastToDialogueDataAsset _returnvalue))
  (bind _output_get (Variables|Default|SetDialogue%20Sequence (Variables|/Script/TypewritterTextTest.DialogueDataAsset|GetDialogueSequence _asdialogue_data_asset)))
  (if (not (Utilities|Array|IsEmpty _output_get))
    (CallFunction|CEonInitDialogue)
    (else
      (Development|PrintString "Dialogue data empty, cannot initialize dialogue" true true "(R=1.000000,G=0.047119,B=0.000000,A=1.000000)"))))

(fn ConstructionScript)